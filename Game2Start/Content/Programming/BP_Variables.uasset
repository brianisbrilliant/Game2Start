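; BP_Variables is a Blueprint sandbox that exercises variables, random values, branching and functions through on-screen debug prints.
; BeginPlay prints a startup message with a random duration, a coin-flip meal choice and a random color name picked by a switch.
; Tick calls UnterwaterCheck, which compares the player character's head socket height to WaterLevel, and prints while underwater.
; A simple AddTwoNumbers helper is defined but unused in these graphs.
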(event `self.ReceiveBeginPlay`
  (bind _returnvalue (`KismetMathLibrary.RandomFloatInRange` 2.0 6.0))
  (`KismetSystemLibrary.PrintString` (`KismetStringLibrary.Concat_StrStr` "Starting Event BeginPlay in the BP_Variables blueprint" "/n" "duration = " (`KismetStringLibrary.Conv_DoubleToString` _returnvalue)) true true (struct :`R` 1.0 :`B` 0.266666 :`A` 0.333) _returnvalue)
  (if (`KismetMathLibrary.RandomBool`)
    (`KismetSystemLibrary.PrintString` "Today we'll eat pizza!")
    (else
      (`KismetSystemLibrary.PrintString` "Today we'll eat Ice Cream")))
  (switch `int` (`KismetMathLibrary.RandomInteger` 5)
    (:`Default`
      (`KismetSystemLibrary.PrintString` "I have no response to that."))
    (:`0`
      (`KismetSystemLibrary.PrintString` "Red"))
    (:`1`
      (`KismetSystemLibrary.PrintString` "Green"))
    (:`2`
      (`KismetSystemLibrary.PrintString` "Blue"))))

(event `self.ReceiveTick`
  (params (DeltaSeconds :type "Float (single-precision)"))
  (if (`self.UnterwaterCheck` (`self.Water Level`))
    (`KismetSystemLibrary.PrintString` "We are Under water" true true (struct :`R` 0.035601 :`G` 0.052861 :`B` 0.768151 :`A` 1.0) DeltaSeconds)))

(fn `AddTwoNumbers`
  (params (FirstNum :type "Float (double-precision)") (SecondNum :type "Float (double-precision)"))
  (returns (Sum :type "Float (double-precision)"))
  (return (+ FirstNum SecondNum)))

(fn `UnterwaterCheck`
  (params (WaterLevel :type "Float (double-precision)"))
  (returns (Underwater :type Boolean))
  (bind (_returnvalue_x _returnvalue_y _returnvalue_z) (`KismetMathLibrary.BreakVector` (`SceneComponent.GetSocketLocation` (`Character.Mesh` (`GameplayStatics.GetPlayerCharacter` 0)) "head")))
  (return (< _returnvalue_z (`local.WaterLevel`))))

(fn `UserConstructionScript`)