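; BP_ProgPickupB is a collectible pickup that awards a random score bonus to the player.
; On BeginPlay a Timeline drives the Cylinder's relative Z to animate it.
; When BP_ThirdPersonCharacter overlaps the Collision component, it adds 5 to 10 points to the Score on the level's single BP_ProgPrac actor, found via GetActorOfClass.
; It then destroys itself and prints the new score.
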(event `self.ReceiveBeginPlay`
  (bind (_direction _newfloattrack) (`Timeline|Timeline`)
    (:`Update`
      (`SceneComponent.K2_SetRelativeLocation` (`self.Cylinder`) (`KismetMathLibrary.MakeVector` 0.0 0.0 (* _newfloattrack 100.0)) false false))))

(event `self.collision.OnComponentBeginOverlap`
  (params (OverlappedComponent :type "PrimitiveComponent Object Reference") (OtherActor :type "Actor Object Reference") (OtherComp :type "PrimitiveComponent Object Reference") (OtherBodyIndex :type Integer) (bFromSweep :type Boolean) (SweepResult :type "HitResult Structure (by ref)"))
  (cast `/Game/ThirdPerson/Blueprints/BP_ThirdPersonCharacter` OtherActor)
  (bind _returnvalue (`GameplayStatics.GetActorOfClass` "/Game/ProgPrac/BP_ProgPrac.BP_ProgPrac_C")) ; There should be only one in the level.
  (bind _output_get (set `/Game/ProgPrac/BP_ProgPrac.Score` (+ (`/Game/ProgPrac/BP_ProgPrac.Score` _returnvalue) (`KismetMathLibrary.RandomIntegerInRange` 5 10)) _returnvalue))
  (`self.K2_DestroyActor`)
  (`KismetSystemLibrary.PrintString` (`KismetStringLibrary.Conv_IntToString` _output_get)))

(fn `UserConstructionScript`)