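; BP_Doorway is a doorway Blueprint that prints a debug string based on its DoorType when its box is overlapped, with no door movement or other behavior.
; The Box begin-overlap event switches on DoorType, printing a number word for each handled value and "broke" for any other.
; An unconnected nested branch chain duplicates the same logic and never runs.
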(event `self.Box.OnComponentBeginOverlap`
  (params (OverlappedComponent :type "PrimitiveComponent Object Reference") (OtherActor :type "Actor Object Reference") (OtherComp :type "PrimitiveComponent Object Reference") (OtherBodyIndex :type Integer) (bFromSweep :type Boolean) (SweepResult :type "HitResult Structure (by ref)"))
  (switch `int` (`self.DoorType`)
    (:`Default`
      (`KismetSystemLibrary.PrintString` "broke"))
    (:`0`
      (`KismetSystemLibrary.PrintString` "zero"))
    (:`1`
      (`KismetSystemLibrary.PrintString` "one"))
    (:`2`
      (`KismetSystemLibrary.PrintString` "two"))))

(fn `UserConstructionScript`)