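; BP_ProcPrac is a practice actor that endlessly spawns BP_ProgPickup actors around itself.
; BeginPlay draws a debug circle, randomizes HasKey, prints score, health, player name and key state, then starts SpawnPickup.
; SpawnPickup repeats through a two-second Delay, placing each pickup at a random horizontal offset scaled by Radius from the root.
; A random pick from the PIckups array is left unused.
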(event `self.ReceiveBeginPlay`
  (`KismetSystemLibrary.DrawDebugCircle` (0.0 0.0 0.0) 500.0 64 (struct :`R` 1.0 :`B` 0.036994 :`A` 1.0) 60.0 5.0 (0.0 1.0 0.0) (1.0 0.0 0.0))
  (set `self.hasKey` (> (`KismetMathLibrary.RandomFloat`) 0.5))
  (`KismetSystemLibrary.PrintString` (`KismetStringLibrary.Concat_StrStr` "Score: " (`KismetStringLibrary.Conv_IntToString` (`self.Score`)) "Health: " (`KismetStringLibrary.Conv_DoubleToString` (`self.Health`)) "Player Name: " (`self.playerName`) "Has Key: " (`KismetStringLibrary.Conv_BoolToString` (`self.hasKey`))))
  (`self.SpawnPickup`))

(event `SpawnPickup`
  (bind _radius (`self.Radius`))
  (`KismetSystemLibrary.Delay` 2.0 :!label _label)
  (`|SpawnActorFromClass` "/Game/ProgPrac/BP_ProgPickup.BP_ProgPickup_C" (`KismetMathLibrary.MakeTransform` (+ (`SceneComponent.K2_GetComponentLocation` (`self.DefaultSceneRoot`)) (* (`KismetMathLibrary.RandomUnitVector`) (`KismetMathLibrary.MakeVector` _radius _radius)))) "Undefined" "MultiplyWithRoot" null null)
  (`self.SpawnPickup`)
  (goto _label))

(fn `UserConstructionScript`)