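; BP_progPickup2 is a score pickup that the third-person character collects by overlapping its sphere.
; A timeline started on BeginPlay moves the cylinder vertically as it plays.
; On overlap it looks up the level's BP_ProgPrac actor, adds a random 5 to 10 to its Score, prints the new total and destroys itself.
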(event `self.ReceiveBeginPlay`
  (bind (_direction _upanddown) (`Timeline|Timeline`)
    (:`Update`
      (`SceneComponent.K2_SetRelativeLocation` (`self.Cylinder`) (`KismetMathLibrary.MakeVector` 0.0 0.0 (+ (* _upanddown 100.0) 50.0)) false false))))

(event `self.Sphere.OnComponentBeginOverlap`
  (params (OverlappedComponent :type "PrimitiveComponent Object Reference") (OtherActor :type "Actor Object Reference") (OtherComp :type "PrimitiveComponent Object Reference") (OtherBodyIndex :type Integer) (bFromSweep :type Boolean) (SweepResult :type "HitResult Structure (by ref)"))
  ;[1 1 1] checking if player is actor that overlaps
  (cast `/Game/ThirdPerson/Blueprints/BP_ThirdPersonCharacter` OtherActor)
  ;[1 1 1] find bp_Progprac in the level
  (bind _returnvalue (`GameplayStatics.GetActorOfClass` "/Game/ProgPrac/BP_ProgPrac.BP_ProgPrac_C"))
  (bind _output_get (set `/Game/ProgPrac/BP_ProgPrac.Score` (+ (`/Game/ProgPrac/BP_ProgPrac.Score` _returnvalue) (`KismetMathLibrary.RandomIntegerInRange` 5 10)) _returnvalue)) ; set number to new score
  (`KismetSystemLibrary.PrintString` (`KismetStringLibrary.Concat_StrStr` "Score: " (`KismetStringLibrary.Conv_IntToString` _output_get)))
  (`self.K2_DestroyActor`) ; destroy this pickup
)

(fn `UserConstructionScript`)