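; BP_progPickupRed is a score pickup whose sphere is animated vertically by the SphereFloat timeline from BeginPlay.
; When a BP_ThirdPersonCharacter overlaps its Collision component, it adds a random amount to the Score variable on the BP_ProgPrac actor found in the level.
; It then prints the new score on screen and destroys itself.
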(event `self.ReceiveBeginPlay`
  (bind (_direction _spherefloat_t) (`Timeline|SphereFloat`)
    (:`Update`
      (`SceneComponent.K2_SetRelativeLocation` (`self.Sphere`) (`KismetMathLibrary.MakeVector` 0.0 0.0 (+ (* _spherefloat_t 50.0) 100.0)) false false))))

(event `self.Collision.OnComponentBeginOverlap`
  (params (OverlappedComponent :type "PrimitiveComponent Object Reference") (OtherActor :type "Actor Object Reference") (OtherComp :type "PrimitiveComponent Object Reference") (OtherBodyIndex :type Integer) (bFromSweep :type Boolean) (SweepResult :type "HitResult Structure (by ref)"))
  (cast `/Game/ThirdPerson/Blueprints/BP_ThirdPersonCharacter` OtherActor)
  (bind _returnvalue (`GameplayStatics.GetActorOfClass` "/Game/ProgPrac/Blueprints/BP_ProgPrac.BP_ProgPrac_C"))
  (bind _output_get (set `/Game/ProgPrac/Blueprints/BP_ProgPrac.Score` (+ (`/Game/ProgPrac/Blueprints/BP_ProgPrac.Score` _returnvalue) (`KismetMathLibrary.RandomIntegerInRange` 5 10)) _returnvalue))
  (`KismetSystemLibrary.PrintString` (`KismetStringLibrary.Concat_StrStr` "Score: " (`KismetStringLibrary.Conv_IntToString` _output_get)) true true (struct :`G` 0.66 :`B` 1.0 :`A` 1.0) 5.0)
  (`self.K2_DestroyActor`))

(fn `UserConstructionScript`)