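; BP_ProgPrac is a programming-practice actor that spawns random pickups around itself and prints debug information.
; On BeginPlay it randomly decides HasKey, prints the player stats, starts spawning and draws a debug circle of the spawn radius.
; SpawnPickup re-calls itself after a short delay, placing a random Pickups class within the flattened radius.
; After each spawn, CheckPopulation prints the count of actors tagged "Pickup".
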(event `self.ReceiveBeginPlay`
  (set `self.HasKey` (> (`KismetMathLibrary.RandomFloat`) 0.75))
  (`KismetSystemLibrary.PrintString` (`KismetStringLibrary.Concat_StrStr` "Player Name: " (`self.PlayerName`) " Health: " (`KismetStringLibrary.Conv_DoubleToString` (`self.Health`)) " Score: " (`KismetStringLibrary.Conv_IntToString` (`self.Score`)) " Has Key? " (`KismetStringLibrary.Conv_BoolToString` (`self.HasKey`))) true true (struct :`G` 0.66 :`B` 1.0 :`A` 1.0) 10.0)
  (`self.SpawnPickup`)
  (`KismetSystemLibrary.DrawDebugCircle` (`SceneComponent.K2_GetComponentLocation` (`self.DefaultSceneRoot`)) (`self.Radius`) 64 (struct :`R` 1.0 :`G` 0.040784 :`A` 1.0) 60.0 30.0 (0.0 1.0 0.0) (1.0 0.0 0.0) true))

(event `SpawnPickup`
  (bind _radius (`self.Radius`))
  (bind _pickups (`self.Pickups`))
  (`|SpawnActorFromClass` (`|GetArrayItem` _pickups (`KismetMathLibrary.RandomIntegerInRange` 0 (- (`KismetArrayLibrary.Array_Length` _pickups) 1))) (`KismetMathLibrary.MakeTransform` (+ (* (`KismetMathLibrary.RandomUnitVector`) (`KismetMathLibrary.MakeVector` _radius _radius)) (`SceneComponent.K2_GetComponentLocation` (`self.DefaultSceneRoot`)))) "Undefined" "MultiplyWithRoot" null null)
  (`self.CheckPopulation`)
  (`KismetSystemLibrary.Delay` 2.0)
  (`self.SpawnPickup`))

(event `CheckPopulation`
  (bind _outactors (`GameplayStatics.GetAllActorsWithTag` "Pickup"))
  (`KismetSystemLibrary.PrintString` (`KismetStringLibrary.Concat_StrStr` "There are " (`KismetStringLibrary.Conv_IntToString` (`KismetArrayLibrary.Array_Length` _outactors)) " pickups.")))

(fn `UserConstructionScript`)