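; BP_Itemm is a base item Blueprint with a physics Cube that can be picked up, dropped and used.
; Pickup turns off the Cube's physics and collision, then after a short delay attaches it to the given parent's left item socket.
; Drop restores collision and physics and applies a forward-upward force, with no detach step.
; PrimaryAction only prints a debug message, and an unconnected loop over child components is left as an open question about their collision.
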(event `Pickup`
  (params (Parent :type "SceneComponent Object Reference"))
  (`KismetSystemLibrary.PrintString` "Picking up")
  (`PrimitiveComponent.SetSimulatePhysics` (`self.Cube`) false)
  (`PrimitiveComponent.SetCollisionEnabled` (`self.Cube`) "NoCollision")
  (`KismetSystemLibrary.Delay` 0.1)
  (`self.K2_AttachToComponent` Parent "item_socket_l" "SnapToTarget" "SnapToTarget" "KeepRelative"))

(event `Drop`
  (`KismetSystemLibrary.PrintString` "Dropping")
  (`PrimitiveComponent.SetCollisionEnabled` (`self.Cube`) "QueryAndPhysics")
  (`PrimitiveComponent.SetSimulatePhysics` (`self.Cube`) true)
  (`PrimitiveComponent.AddForce` (`self.Cube`) (500.0 0.0 300.0) "None" false))

(event `Primary Action`
  (`KismetSystemLibrary.PrintString` "Primary Action"))

(fn `UserConstructionScript`)