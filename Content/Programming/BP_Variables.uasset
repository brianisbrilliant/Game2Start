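; BP_Variables is a sandbox actor that demonstrates variable types and branching through on-screen debug prints.
; BeginPlay prints a start message with random duration, picks pizza or ice cream from a random bool, then switches on a random integer for colour names or a fallback.
; Tick reports being under water, for one frame at a time, whenever the player's head socket is below a fixed world height.
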(event `self.ReceiveBeginPlay`
  (bind _returnvalue (`KismetMathLibrary.RandomFloatInRange` 2.0 6.0))
  (`KismetSystemLibrary.PrintString` (`KismetStringLibrary.Concat_StrStr` "Starting Event BeginPlay in the BP_Variables blueprint" "/n" "duration = " (`KismetStringLibrary.Conv_DoubleToString` _returnvalue)) true true (struct :`R` 1.0 :`B` 0.266666 :`A` 0.333) _returnvalue)
  (if (`KismetMathLibrary.RandomBool`)
    (`KismetSystemLibrary.PrintString` "Today we'll eat pizza!")
    (else
      (`KismetSystemLibrary.PrintString` "Today we'll eat Ice Cream")))
  (switch `int` (`KismetMathLibrary.RandomInteger` 5)
    (:`Default`
      (`KismetSystemLibrary.PrintString` "I have no response to that."))
    (:`0`
      (`KismetSystemLibrary.PrintString` "Red"))
    (:`1`
      (`KismetSystemLibrary.PrintString` "Green"))
    (:`2`
      (`KismetSystemLibrary.PrintString` "Blue"))))

(event `self.ReceiveTick`
  (params (DeltaSeconds :type "Float (single-precision)"))
  (bind (_returnvalue_x _returnvalue_y _returnvalue_z) (`KismetMathLibrary.BreakVector` (`SceneComponent.GetSocketLocation` (`Character.Mesh` (`GameplayStatics.GetPlayerCharacter` 0)) "head")))
  (if (< _returnvalue_z 300.0)
    (`KismetSystemLibrary.PrintString` "We are Under water" true true (struct :`G` 0.66 :`B` 1.0 :`A` 1.0) DeltaSeconds)))

(fn `UserConstructionScript`)