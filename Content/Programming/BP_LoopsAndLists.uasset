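; BP_LoopsAndLists is an actor, apparently a loops and lists exercise, that spawns and counts a configurable actor class.
; It enables player input on BeginPlay, and the N key spawns an ActorToSpawn at a random horizontal offset around its root.
; A self-calling CheckRemaining event counts those actors, printing the total after a short delay while under ten.
; Nothing in this graph starts that check.
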(event `self.ReceiveBeginPlay`
  (`self.EnableInput` (`GameplayStatics.GetPlayerController` 0)))

(event `SpawnNewThing`
  (bind _returnvalue (`KismetMathLibrary.RandomFloatInRange` 200.0 4000.0))
  (`|SpawnActorFromClass` (`self.ActorToSpawn`) (`KismetMathLibrary.MakeTransform` (+ (`SceneComponent.K2_GetComponentLocation` (`self.DefaultSceneRoot`)) (* (`KismetMathLibrary.RandomUnitVector`) (`KismetMathLibrary.MakeVector` _returnvalue _returnvalue)))) "Undefined" "MultiplyWithRoot" null null))

(event `Check Remaining`
  (bind _outactors (`GameplayStatics.GetAllActorsOfClass` (`self.ActorToSpawn`)))
  (bind _returnvalue (`KismetArrayLibrary.Array_Length` _outactors))
  (if (< _returnvalue 10)
    (`KismetSystemLibrary.Delay` 0.2)
    (`KismetSystemLibrary.PrintString` (`KismetStringLibrary.Concat_StrStr` "There are " (`KismetStringLibrary.Conv_IntToString` _returnvalue) (`KismetSystemLibrary.GetClassDisplayName` (`self.ActorToSpawn`)) " in the level.") true true (struct :`G` 0.66 :`B` 1.0 :`A` 1.0) 0.2))
  (`self.Check Remaining`))

(event `Key|N`
  (params (Key :type "Key Structure"))
  (:`Pressed`
    (`self.SpawnNewThing`)))

(fn `UserConstructionScript`)