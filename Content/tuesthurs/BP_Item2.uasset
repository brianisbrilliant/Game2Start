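; BP_Item2 is an item actor that a character can pick up and drop, with a placeholder primary action that only prints.
; Pickup, gated by CanBePickedUp, disables Cube collision and attaches the item to the given skeletal mesh's item_socket_r.
; Drop detaches it, restores collision, enables physics and applies a fixed force to the Cube.
; After a short delay it stops simulating and allows pickup again.
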(event `pickup`
  (params (SkeletalMesh :type "SceneComponent Object Reference"))
  (if (`self.CanBePickedUp`)
    (set `self.CanBePickedUp` false)
    (`KismetSystemLibrary.PrintString` "calling pickup" true true (struct :`G` 1.0 :`B` 0.058931 :`A` 1.0) 6.0)
    (`PrimitiveComponent.SetCollisionEnabled` (`self.Cube`) "NoCollision")
    (`self.K2_AttachToComponent` SkeletalMesh "item_socket_r" "SnapToTarget" "SnapToTarget" "KeepRelative")
    (else
      (`KismetSystemLibrary.PrintString` "in cooldown"))))

(event `drop`
  (`KismetSystemLibrary.PrintString` "calling drop" true true (struct :`R` 1.0 :`B` 0.109308 :`A` 1.0) 4.0)
  (`SceneComponent.K2_DetachFromComponent` (`self.Cube`) "KeepWorld" "KeepWorld" "KeepWorld" true)
  (`PrimitiveComponent.SetSimulatePhysics` (`self.Cube`) true)
  (`self.K2_DetachFromActor` self "KeepWorld" "KeepWorld" "KeepRelative")
  (`PrimitiveComponent.SetCollisionEnabled` (`self.Cube`) "QueryAndPhysics")
  (`PrimitiveComponent.AddForce` (`self.Cube`) (500.0 0.0 250.0) "None" false)
  (`KismetSystemLibrary.Delay` 4.0)
  (set `self.CanBePickedUp` true)
  (`PrimitiveComponent.SetSimulatePhysics` (`self.Cube`) false))

(event `primaryAction`
  (`KismetSystemLibrary.PrintString` "Calling primary action"))

(fn `UserConstructionScript`)