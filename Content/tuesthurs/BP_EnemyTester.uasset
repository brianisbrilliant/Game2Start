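; BP_EnemyTester is a test actor that repeatedly damages every BP_Enemy2 in the level.
; From BeginPlay, it gathers all BP_Enemy2 actors, prints their count, and calls TakeDamage on each with a small random amount, printing each array index.
; After a confirmation message and a short Delay, the GiveDamage event calls itself, repeating the search and damage pass indefinitely.
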(event `GiveDamage`
  (bind _outactors (`GameplayStatics.GetAllActorsOfClass` "/Game/tuesthurs/BP_Enemy2.BP_Enemy2_C" :!label _label)) ; find all of the BP_enemies
  (`KismetSystemLibrary.PrintString` (`KismetStringLibrary.Concat_StrStr` "There are " (`KismetStringLibrary.Conv_IntToString` (`KismetArrayLibrary.Array_Length` _outactors)) " enemies in the level."))
  (for (_array_element _array_index) _outactors
    (`/Game/tuesthurs/BP_Enemy2.TakeDamage` _array_element (`KismetMathLibrary.RandomFloatInRange` 0.1 0.5))
    (`KismetSystemLibrary.PrintString` (`KismetStringLibrary.Concat_StrStr` "array index = " (`KismetStringLibrary.Conv_IntToString` _array_index)) true true (struct :`G` 0.66 :`B` 1.0 :`A` 1.0) 5.0))
  (`KismetSystemLibrary.PrintString` "We've given Damage to all of the enemies.")
  (`KismetSystemLibrary.Delay` 2.0)
  (`self.GiveDamage`))

(event `self.ReceiveBeginPlay`
  (goto _label))

(fn `UserConstructionScript`)