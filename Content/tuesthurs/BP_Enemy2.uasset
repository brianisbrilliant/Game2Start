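; BP_Enemy2 is a simple damageable enemy Blueprint that prints a threat message when play begins.
; Its TakeDamage event prints a reaction, subtracts the amount from Health and destroys the actor once CheckIfDead reports Health at zero or below.
; It has no movement or attack logic, and its construction script is empty.
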(event `self.ReceiveBeginPlay`
  (`KismetSystemLibrary.PrintString` "Hello, I have been programmed to destroy you."))

(event `TakeDamage`
  (params (ByAmount :type "Float (double-precision)" :default 0.2))
  (`KismetSystemLibrary.PrintString` "Ouch!")
  (set `self.health` (- (`self.health`) ByAmount))
  (if (`self.CheckIfDead` (`self.health`))
    (`self.K2_DestroyActor`)))

(fn `CheckIfDead`
  (params (Health :type "Float (double-precision)"))
  (returns (IsDead :type Boolean))
  (return (<= Health 0.0)))

(fn `UserConstructionScript`)