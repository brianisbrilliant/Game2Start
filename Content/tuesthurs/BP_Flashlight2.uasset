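; BP_Flashlight2 is a flashlight actor whose logic consists of a state toggle and debug output, with no light control in its graphs.
; PrimaryAction prints ON or OFF from FlashlightOn, then flips it, so the message shows the state before the toggle.
; Tick prints the Cube's physics simulation and collision state and draws a debug box at its location.
; A second debug box at DefaultSceneRoot is disconnected.
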(event `self.primaryAction`
  (if (`self.FlashlightOn`)
    (`KismetSystemLibrary.PrintString` "FLASHLIGHT ON" true true (struct :`G` 0.107174 :`B` 1.0 :`A` 1.0))
    (else
      (`KismetSystemLibrary.PrintString` "FLASHLIGHT OFF" true true (struct :`R` 1.0 :`G` 0.308648 :`A` 1.0))))
  (set `self.FlashlightOn` (not (`self.FlashlightOn`))))

(event `self.ReceiveTick`
  (params (DeltaSeconds :type "Float (single-precision)"))
  (if (`SceneComponent.IsSimulatingPhysics` (`self.Cube`) "None")
    (`KismetSystemLibrary.PrintString` "Physics active" true true (struct :`R` 1.0 :`G` 0.870101 :`A` 1.0) DeltaSeconds)
    (else
      (`KismetSystemLibrary.PrintString` "Physics inactive" true true (struct :`R` 1.0 :`B` 0.852574 :`A` 1.0) DeltaSeconds)))
  (`KismetSystemLibrary.PrintString` (`|GetEnumeratorNameAsString` (`PrimitiveComponent.GetCollisionEnabled` (`self.Cube`))) true true (struct :`G` 0.66 :`B` 1.0 :`A` 1.0) DeltaSeconds)
  (`KismetSystemLibrary.DrawDebugBox` (`SceneComponent.K2_GetComponentLocation` (`self.Cube`)) (40.0 40.0 40.0) (struct :`R` 1.0 :`B` 0.187314 :`A` 1.0) (struct) 0.0 10.0))

(fn `UserConstructionScript`
  (`parent.UserConstructionScript`))