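; Test actor with a physics sphere that repeatedly throws itself and records its trajectory to a CSV file.
; A loop applies a random-direction impulse, waits, then resets the sphere to its start position with zeroed velocities and throws again.
; A parallel self-calling delay loop samples its world position as comma-separated strings.
; Five seconds after BeginPlay, the samples are written once to a hardcoded local path, with the result printed.
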(event `self.ReceiveBeginPlay`
  (set `self.OriginalLocation` (`SceneComponent.K2_GetComponentLocation` (`self.Sphere`)))
  (`self.Throw Ball`)
  (`self.StoreLocation`)
  (`KismetSystemLibrary.Delay` 5.0)
  (`self.Save to File`))

(event `Throw Ball`
  (`PrimitiveComponent.AddImpulse` (`self.Sphere`) (* (`KismetMathLibrary.RandomUnitVector`) 5000.0) "None" false)
  (`KismetSystemLibrary.Delay` 3.0)
  (`self.Reset Ball`))

(event `Reset Ball`
  (`SceneComponent.K2_SetWorldLocation` (`self.Sphere`) (`self.OriginalLocation`) false false)
  (`PrimitiveComponent.SetAllPhysicsLinearVelocity` (`self.Sphere`) (0.0 0.0 0.0) false)
  (`PrimitiveComponent.SetAllPhysicsAngularVelocityInDegrees` (`self.Sphere`) (`KismetMathLibrary.Vector_Zero`) false)
  (`self.Throw Ball`))

(event `StoreLocation`
  (bind (_returnvalue_x _returnvalue_y _returnvalue_z) (`KismetMathLibrary.BreakVector` (`SceneComponent.K2_GetComponentLocation` (`self.Sphere`))))
  (`KismetArrayLibrary.Array_Add` (`self.StringLocations`) (`KismetStringLibrary.Concat_StrStr` (`KismetStringLibrary.Conv_DoubleToString` _returnvalue_x) "," (`KismetStringLibrary.Conv_DoubleToString` _returnvalue_y) "," (`KismetStringLibrary.Conv_DoubleToString` _returnvalue_z) "\\n"))
  (`KismetSystemLibrary.Delay` 0.5)
  (`self.StoreLocation`))

(event `Save to File`
  (bind _returnvalue (`VictoryBPFunctionLibrary.FileIO__SaveStringArrayToFile` "C:\\cpp" "savedlocations.csv" (`self.StringLocations`) true))
  (if _returnvalue
    (`KismetSystemLibrary.PrintString` "File Saved Successfully!")
    (else
      (`KismetSystemLibrary.PrintString` "Unable to Save File"))))

(event `Save Locations`)

(fn `UserConstructionScript`)