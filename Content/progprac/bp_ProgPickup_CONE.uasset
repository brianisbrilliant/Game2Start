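; A cone pickup actor that adds a random amount of points when the third-person character touches it.
; A timeline started on BeginPlay moves the cone mesh's relative height to make it float.
; On hitbox overlap, it finds the Bp_ProgPrac actor by class, increases its Score, then destroys itself.
; An unconnected node chain for randomly offsetting the actor's location never runs.
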(event `self.ReceiveBeginPlay`
  (bind (_direction _floating) (`Timeline|Timeline`)
    (:`Update`
      (`SceneComponent.K2_SetRelativeLocation` (`self.Cone`) (`KismetMathLibrary.MakeVector` 0.0 0.0 (* _floating 10.0)) false false))))

(event `self.Hitbox.OnComponentBeginOverlap`
  (params (OverlappedComponent :type "PrimitiveComponent Object Reference") (OtherActor :type "Actor Object Reference") (OtherComp :type "PrimitiveComponent Object Reference") (OtherBodyIndex :type Integer) (bFromSweep :type Boolean) (SweepResult :type "HitResult Structure (by ref)"))
  (cast `/Game/ThirdPerson/Blueprints/BP_ThirdPersonCharacter` OtherActor)
  (bind _returnvalue (`GameplayStatics.GetActorOfClass` "/Game/progprac/bp_ProgPrac.bp_ProgPrac_C"))
  (set `/Game/progprac/bp_ProgPrac.Score` (+ (`/Game/progprac/bp_ProgPrac.Score` _returnvalue) (`KismetMathLibrary.RandomIntegerInRange` 5 10)) _returnvalue)
  (`self.K2_DestroyActor`))

(fn `UserConstructionScript`)