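; BP_progprac is a practice Blueprint that randomizes a key flag, prints player stats and repeatedly spawns actors around itself.
; On BeginPlay it gives HasKey a one-in-four chance of being true, prints score, health, name and key state, then calls SpawnPickup.
; SpawnPickup loops endlessly on a short delay, spawning at a random horizontal offset from its root with the player character as instigator.
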(event `SpawnPickup`
  (params (SpawnTransform :type "Transform Structure"))
  (`|SpawnActorFromClass` "/Game/Blueprints/BP_progPickup.BP_progPickup_C" (`KismetMathLibrary.MakeTransform` (+ (`SceneComponent.K2_GetComponentLocation` (`self.DefaultSceneRoot`)) (* (`KismetMathLibrary.RandomUnitVector`) (500.0 500.0 0.0)))) "Undefined" "MultiplyWithRoot" null (`GameplayStatics.GetPlayerCharacter` 0) :!label _label)
  (`KismetSystemLibrary.Delay` 2.0)
  (goto _label))

(event `self.ReceiveBeginPlay`
  (`|ExecutionSequence`
    (:`then_0`
      (set `self.hasKey` (>= (`KismetMathLibrary.RandomFloat`) 0.75)))
    (:`then_1`
      (`KismetSystemLibrary.PrintString` (`KismetStringLibrary.Concat_StrStr` "score =  " (`KismetStringLibrary.Conv_IntToString` (`self.score`)) "  health  " (`KismetStringLibrary.Conv_DoubleToString` (`self.health`)) "  player name:  " (`self.playerName`) "  has key? " (`KismetStringLibrary.Conv_BoolToString` (`self.hasKey`))) true true (struct :`G` 0.66 :`B` 1.0 :`A` 1.0) 10.0))
    (:`then_2`
      (`self.SpawnPickup` (struct)))))

(event `self.ReceiveTick`
  (params (DeltaSeconds :type "Float (single-precision)")))

(fn `UserConstructionScript`)