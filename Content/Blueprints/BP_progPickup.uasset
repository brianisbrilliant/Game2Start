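; BP_progPickup is a pickup whose Cylinder moves along Z by a Timeline curve started on BeginPlay.
; When BP_ThirdPersonCharacter overlaps its Capsule, it adds a random 5 to 10 points to the Score on the BP_progprac found via GetActorOfClass.
; It then destroys itself and prints the new score.
; The actor-level overlap event only casts and does nothing further.
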(event `self.ReceiveBeginPlay`
  (bind (_direction _anim_cylinder) (`Timeline|Timeline`)
    (:`Update`
      (`SceneComponent.K2_SetRelativeLocation` (`self.Cylinder`) (`KismetMathLibrary.MakeVector` 0.0 0.0 (* _anim_cylinder 100.0)) false false))))

(event `self.ReceiveActorBeginOverlap`
  (params (OtherActor :type "Actor Object Reference"))
  (cast `/Game/ThirdPerson/Blueprints/BP_ThirdPersonCharacter` OtherActor))

(event `self.Capsule.OnComponentBeginOverlap`
  (params (OverlappedComponent :type "PrimitiveComponent Object Reference") (OtherActor :type "Actor Object Reference") (OtherComp :type "PrimitiveComponent Object Reference") (OtherBodyIndex :type Integer) (bFromSweep :type Boolean) (SweepResult :type "HitResult Structure (by ref)"))
  (cast `/Game/ThirdPerson/Blueprints/BP_ThirdPersonCharacter` OtherActor)
  (bind _returnvalue (`GameplayStatics.GetActorOfClass` "/Game/Blueprints/BP_progprac.BP_progprac_C")) ; useful
  (bind _output_get (set `/Game/Blueprints/BP_progprac.score` (+ (`/Game/Blueprints/BP_progprac.score` _returnvalue) (`KismetMathLibrary.RandomIntegerInRange` 5 10)) _returnvalue))
  (`self.K2_DestroyActor`)
  (`KismetSystemLibrary.PrintString` (`KismetStringLibrary.Conv_IntToString` _output_get)))

(fn `UserConstructionScript`)