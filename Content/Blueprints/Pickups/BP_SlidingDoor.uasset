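; BP_SlidingDoor is a door that opens by sliding along its Z axis when a qualifying actor enters its Box trigger.
; Overlap start spawns a looping sound at the actor's root and plays the OpenDoor timeline, which drives the Door's relative Z location.
; Overlap end reverses the timeline from its end to close the door.
; The sound stops whenever the timeline finishes.
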(event `self.Box.OnComponentBeginOverlap`
  (params (OverlappedComponent :type "PrimitiveComponent Object Reference") (OtherActor :type "Actor Object Reference") (OtherComp :type "PrimitiveComponent Object Reference") (OtherBodyIndex :type Integer) (bFromSweep :type Boolean) (SweepResult :type "HitResult Structure (by ref)"))
  (cast `` OtherActor)
  (`|ExecutionSequence`
    (:`then_0`
      (bind _returnvalue (`GameplayStatics.SpawnSoundAtLocation` "/Game/Audio/HitHurt5Looping.HitHurt5Looping" (`SceneComponent.K2_GetComponentLocation` (`self.DefaultSceneRoot`)) (struct) 1.0 0.01 0.0 null null false)))
    (:`then_1`
      (bind (_direction _newtrack_0) (`Timeline|OpenDoor` :!label _label)
        (:`Update`
          (`SceneComponent.K2_SetRelativeLocation` (`self.Door`) (`KismetMathLibrary.MakeVector` 0.0 0.0 (* _newtrack_0 270.0)) false false))
        (:`Finished`
          (`/Engine/EditorBlueprintResources/StandardMacros.IsValid` _returnvalue
            (:`Is Valid`
              (`AudioComponent.Stop` _returnvalue))))))))

(event `self.Box.OnComponentEndOverlap`
  (params (OverlappedComponent :type "PrimitiveComponent Object Reference") (OtherActor :type "Actor Object Reference") (OtherComp :type "PrimitiveComponent Object Reference") (OtherBodyIndex :type Integer))
  (cast `` OtherActor)
  (goto _label :!via `ReverseFromEnd`))

(fn `UserConstructionScript`)