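; Blueprint platform that alternates between moving up and down when the third-person character overlaps its trigger.
; PlatformUp selects one of two timelines, each lerping the platform's relative location between the Start and End component locations.
; Each timeline flips the PlatformUp and PlatformDown flags only on finishing, so re-entering mid-move restarts that same move from its beginning.
; Debug strings print the direction of travel.
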(event `self.ReceiveBeginPlay`)

(event `self.Trigger.OnComponentBeginOverlap`
  (params (OverlappedComponent :type "PrimitiveComponent Object Reference") (OtherActor :type "Actor Object Reference") (OtherComp :type "PrimitiveComponent Object Reference") (OtherBodyIndex :type Integer) (bFromSweep :type Boolean) (SweepResult :type "HitResult Structure (by ref)"))
  (cast `/Game/ThirdPerson/Blueprints/BP_ThirdPersonCharacter` OtherActor)
  (if (`self.PlatformUp`)
    (`KismetSystemLibrary.PrintString` "playform moving down ")
    (bind (_direction _newtrack_0) (`Timeline|Timeline_1` :!via `PlayFromStart`)
      (:`Update`
        (`SceneComponent.K2_SetRelativeLocation` (`self.Platform`) (`KismetMathLibrary.VLerp` (`SceneComponent.RelativeLocation` (`self.Start`)) (`SceneComponent.RelativeLocation` (`self.End`)) _newtrack_0) false false))
      (:`Finished`
        (set `self.PlatformUp` false)
        (set `self.PlatformDown` true)))
    (else
      (`KismetSystemLibrary.PrintString` "playform moving up ")
      (bind (_direction_2 _newtrack_0_2) (`Timeline|Timeline` :!via `PlayFromStart`)
        (:`Update`
          (`SceneComponent.K2_SetRelativeLocation` (`self.Platform`) (`KismetMathLibrary.VLerp` (`SceneComponent.RelativeLocation` (`self.Start`)) (`SceneComponent.RelativeLocation` (`self.End`)) _newtrack_0_2) false false))
        (:`Finished`
          (set `self.PlatformUp` true)
          (set `self.PlatformDown` false))))))

(fn `UserConstructionScript`)