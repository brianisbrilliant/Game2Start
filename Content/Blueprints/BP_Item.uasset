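; BP_Item is a holdable item actor with pick-up, drop and primary-action events.
; PickUp runs while CanPickup is true, clearing it, disabling Cube collision and snapping to the passed skeletal mesh's handitem_r socket.
; Drop restores collision, detaches, enables physics and tosses the Cube along a fixed world-space force, but leaves CanPickup false.
; PrimaryAction only prints a debug string.
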(event `PickUp`
  (params (SKMesh :type "SceneComponent Object Reference"))
  (if (`self.canPickup`)
    (set `self.canPickup` false)
    (`KismetSystemLibrary.PrintString` "picked up")
    (`PrimitiveComponent.SetCollisionEnabled` (`self.Cube`) "NoCollision")
    (`self.K2_AttachToComponent` SKMesh "handitem_r" "SnapToTarget" "KeepRelative" "KeepRelative")))

(event `Drop`
  (bind _cube (`self.Cube`))
  (`KismetSystemLibrary.PrintString` "dropped")
  (`PrimitiveComponent.SetCollisionEnabled` (`self.Cube`) "QueryAndPhysics")
  (`self.K2_DetachFromActor` "KeepWorld" "KeepWorld")
  (`PrimitiveComponent.SetSimulatePhysics` _cube true)
  (`PrimitiveComponent.AddForce` _cube (500.0 0.0 250.0) "None" true))

(event `PrimaryAction`
  (`KismetSystemLibrary.PrintString` "primary action!!!"))

(fn `UserConstructionScript`)