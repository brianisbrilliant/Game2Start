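; BP_TeleportStaff is an item that randomly teleports the player character when its primary action is used.
; PrimaryAction moves the BP_ThirdPersonCharacter found by class lookup along a random direction scaled by Radius on X and Y only, keeping height, and randomizes its yaw.
; It prints a "POOF!" message and spawns a Niagara effect just below the character at the new position.
; A CanUse flag with a short delay acts as a cooldown.
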(event `self.PrimaryAction`
  (bind _radius (`self.Radius`))
  (if (`self.canUse`)
    (set `self.canUse` false)
    (`KismetSystemLibrary.PrintString` "POOF!" true true (struct :`R` 0.367118 :`G` 0.094948 :`B` 1.0 :`A` 1.0))
    (bind _returnvalue (`GameplayStatics.GetActorOfClass` "/Game/ThirdPerson/Blueprints/BP_ThirdPersonCharacter.BP_ThirdPersonCharacter_C"))
    (`self.K2_SetActorLocationAndRotation` _returnvalue (+ (* (`KismetMathLibrary.RandomUnitVector`) (`KismetMathLibrary.MakeVector` _radius _radius)) (`self.K2_GetActorLocation` _returnvalue)) (`KismetMathLibrary.MakeRotator` 0.0 0.0 (`KismetMathLibrary.RandomFloatInRange` 40.0 300.0)) false false)
    (`NiagaraFunctionLibrary.SpawnSystemAtLocation` "/Game/VFX/CheckpointSystem.CheckpointSystem" (- (`self.K2_GetActorLocation` _returnvalue) (0.0 0.0 50.0)))
    (`KismetSystemLibrary.Delay` 1.0)
    (set `self.canUse` true)))

(fn `UserConstructionScript`
  (`parent.UserConstructionScript`))