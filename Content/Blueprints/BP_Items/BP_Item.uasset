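; BP_Item is a physical item that can be picked up, held and thrown, with a primary action that only prints a debug message.
; PickUp disables physics and collision and snaps the Cube component to the passed skeletal mesh's right-hand socket.
; Drop detaches it, teleports it to the head socket and launches it forward and up from player zero's facing, then turns physics off after a short delay.
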(event `PickUp`
  (params (SKMesh :type "SceneComponent Object Reference"))
  (`PrimitiveComponent.SetSimulatePhysics` (`self.Cube`) false)
  (`KismetSystemLibrary.PrintString` "picked up" true true (struct :`G` 1.0 :`B` 0.048745 :`A` 1.0))
  (`self.SetActorEnableCollision` false)
  (`SceneComponent.K2_AttachToComponent` (`self.Cube`) SKMesh "handitem_r" "SnapToTarget" "SnapToTarget" "KeepRelative" true))

(event `Drop`
  (`SceneComponent.K2_DetachFromComponent` (`self.Cube`) "KeepWorld" "KeepWorld" "KeepRelative" true)
  (`self.K2_SetActorLocation` (`SceneComponent.GetSocketLocation` (stale `PickUp` SKMesh) "head") false true)
  (`self.SetActorEnableCollision` true)
  (`PrimitiveComponent.SetSimulatePhysics` (`self.Cube`) true)
  (`PrimitiveComponent.AddImpulse` (`self.Cube`) (+ (* (`self.GetActorForwardVector` (`GameplayStatics.GetPlayerCharacter` 0)) 250.0) (0.0 0.0 500.0)) "None" true)
  (`KismetSystemLibrary.Delay` 2.0)
  (`PrimitiveComponent.SetSimulatePhysics` (`self.Cube`) false))

(event `PrimaryAction`
  (`KismetSystemLibrary.PrintString` "primary action!!!"))

(fn `UserConstructionScript`)