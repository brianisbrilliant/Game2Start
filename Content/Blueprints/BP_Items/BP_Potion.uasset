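; BP_Potion is a drinkable item that applies a random temporary effect to the player character.
; PrimaryAction prints a chug message and picks one of three effects: very slow walking, very fast walking or a flipped actor rotation.
; After a short delay it writes back hard-coded walk speed or zero rotation rather than saved values.
; A CanDrink flag blocks drinking again until the effect ends.
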(event `self.PrimaryAction`
  (bind _returnvalue (`GameplayStatics.GetPlayerCharacter` 0))
  (bind _charactermovement (`Character.CharacterMovement` (`GameplayStatics.GetPlayerCharacter` 0)))
  (bind _charactermovement_2 (`Character.CharacterMovement` (`GameplayStatics.GetPlayerCharacter` 0)))
  (if (`self.canDrink`)
    (set `self.canDrink` false)
    (`KismetSystemLibrary.PrintString` "CHUG CHUG CHUG CHUG!!!")
    (switch `int` (`KismetMathLibrary.RandomIntegerInRange` 0 2)
      (:`0`
        (set `CharacterMovementComponent.MaxWalkSpeed` 50.0 _charactermovement_2)
        (`KismetSystemLibrary.Delay` 3.0)
        (set `CharacterMovementComponent.MaxWalkSpeed` 600.0 _charactermovement_2))
      (:`1`
        (set `CharacterMovementComponent.MaxWalkSpeed` 4000.0 _charactermovement)
        (`KismetSystemLibrary.Delay` 3.0)
        (set `CharacterMovementComponent.MaxWalkSpeed` 600.0 _charactermovement))
      (:`2`
        (`self.K2_SetActorRotation` _returnvalue (struct :`Roll` 180.0) false)
        (`KismetSystemLibrary.Delay` 3.0)
        (`self.K2_SetActorRotation` :`self` _returnvalue)))
    (set `self.canDrink` true)))

(fn `UserConstructionScript`
  (`parent.UserConstructionScript`))