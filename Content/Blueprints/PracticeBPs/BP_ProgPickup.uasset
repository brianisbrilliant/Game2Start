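; BP_ProgPickup is a practice pickup that awards a random score bonus when the third-person character overlaps it.
; A Timeline started on BeginPlay animates the Cone's relative height, restarting on finish through a zero-length Delay to loop.
; Sphere overlap by BP_ThirdPersonCharacter calls Pickup, which finds BP_ProgPrac with GetActorOfClass, increases its Score, then destroys the pickup.
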(event `self.ReceiveBeginPlay`
  (bind (_direction _newtrack_0) (`Timeline|Timeline` :!label _label)
    (:`Update`
      (`SceneComponent.K2_SetRelativeLocation` (`self.Cone`) (`KismetMathLibrary.MakeVector` 0.0 0.0 (+ (* _newtrack_0 100.0) 50.0)) false false))
    (:`Finished`
      (`KismetSystemLibrary.Delay` 0.0)
      (goto _label :!via `PlayFromStart`))))

(event `self.Sphere.OnComponentBeginOverlap`
  (params (OverlappedComponent :type "PrimitiveComponent Object Reference") (OtherActor :type "Actor Object Reference") (OtherComp :type "PrimitiveComponent Object Reference") (OtherBodyIndex :type Integer) (bFromSweep :type Boolean) (SweepResult :type "HitResult Structure (by ref)"))
  (cast `/Game/ThirdPerson/Blueprints/BP_ThirdPersonCharacter` OtherActor)
  (`self.Pickup`))

(event `Pickup`
  (bind _returnvalue (`GameplayStatics.GetActorOfClass` "/Game/Blueprints/PracticeBPs/BP_ProgPrac.BP_ProgPrac_C"))
  (set `/Game/Blueprints/PracticeBPs/BP_ProgPrac.Score` (+ (`/Game/Blueprints/PracticeBPs/BP_ProgPrac.Score` _returnvalue) (`KismetMathLibrary.RandomIntegerInRange` 5 10)) _returnvalue)
  (`self.K2_DestroyActor`))

(fn `UserConstructionScript`)