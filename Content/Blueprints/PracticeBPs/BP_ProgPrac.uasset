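; BP_ProgPrac is a practice actor that spawns BP_ProgPickup actors around itself and prints player-style stats.
; BeginPlay gives a 25% chance of a key, draws a debug circle at the spawn radius and starts two looping Delay chains.
; One loop spawns pickups at random XY offsets within the radius; the other refreshes the stats and checks pickup count.
; At five or more pickups, a DoOnce-gated Sequence spawns a five-pickup burst, then resets after a delay.
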(event `self.ReceiveBeginPlay`
  (`KismetSystemLibrary.PrintString` (`KismetStringLibrary.Concat_StrStr` "Score: " (`KismetStringLibrary.Conv_IntToString` (`self.Score`)) "  Health: " (`KismetStringLibrary.Conv_DoubleToString` (`self.Health`)) "  Name: " (`self.PlayerName`) "  Key: " (`KismetStringLibrary.Conv_BoolToString` (`self.HasKey`))) true true (struct :`G` 0.176122 :`B` 1.0 :`A` 1.0) 10.0 "1")
  (if (> (`KismetMathLibrary.RandomIntegerInRange` 1 100) 75)
    (set `self.HasKey` true)
    (`KismetSystemLibrary.PrintString` "You have obtained a key!" true true (struct :`G` 0.366667 :`B` 0.003936 :`A` 1.0) 10.0))
  (`self.PrintAtt`)
  (`self.SpawnPickup`)
  (`KismetSystemLibrary.DrawDebugCircle` (`SceneComponent.K2_GetComponentLocation` (`self.DefaultSceneRoot`)) (`self.Radius`) 64 (struct :`R` 1.0 :`G` 1.0 :`B` 1.0 :`A` 1.0) 100000.0 50.0 (0.0 1.0 0.0) (1.0 0.0 0.0) true))

(event `PrintAtt`
  (`KismetSystemLibrary.PrintString` (`KismetStringLibrary.Concat_StrStr` "Score: " (`KismetStringLibrary.Conv_IntToString` (`self.Score`)) "  Health: " (`KismetStringLibrary.Conv_DoubleToString` (`self.Health`)) "  Name: " (`self.PlayerName`) "  Key: " (`KismetStringLibrary.Conv_BoolToString` (`self.HasKey`))) true true (struct :`G` 0.176122 :`B` 1.0 :`A` 1.0) 10.0 "1" :!label _label)
  (`self.CheckPopulation`)
  (`KismetSystemLibrary.Delay` 0.2)
  (goto _label))

(event `SpawnPickup`
  (bind _radius (`self.Radius`))
  (`|SpawnActorFromClass` "/Game/Blueprints/PracticeBPs/BP_ProgPickup.BP_ProgPickup_C" (`KismetMathLibrary.MakeTransform` (+ (`SceneComponent.K2_GetComponentLocation` (`self.DefaultSceneRoot`)) (* (`KismetMathLibrary.RandomUnitVector`) (`KismetMathLibrary.MakeVector` _radius _radius)))) "Undefined" "MultiplyWithRoot" null null :!label _label_2)
  (`KismetSystemLibrary.Delay` 1.25)
  (goto _label_2))

(event `CheckPopulation`
  (bind _radius (`self.Radius`))
  (bind _outactors (`GameplayStatics.GetAllActorsOfClass` "/Game/Blueprints/PracticeBPs/BP_ProgPickup.BP_ProgPickup_C"))
  (if (>= (`KismetArrayLibrary.Array_Length` _outactors) 5)
    (`/Engine/EditorBlueprintResources/StandardMacros.DoOnce` false :!label _label_3
      (:`Completed`
        (`|ExecutionSequence`
          (:`then_0`
            _)
          (:`then_1`
            _)
          (:`then_2`
            _)
          (:`then_3`
            _)
          (:`then_4`
            _)
          (:`then_5`
            (`KismetSystemLibrary.Delay` 10.0)
            (goto _label_3 :!via `Reset`)))
        (`|SpawnActorFromClass` "/Game/Blueprints/PracticeBPs/BP_ProgPickup.BP_ProgPickup_C" (`KismetMathLibrary.MakeTransform` (+ (`SceneComponent.K2_GetComponentLocation` (`self.DefaultSceneRoot`)) (* (`KismetMathLibrary.RandomUnitVector`) (`KismetMathLibrary.MakeVector` _radius _radius)))) "Undefined" "MultiplyWithRoot" null null)))))

(fn `UserConstructionScript`)