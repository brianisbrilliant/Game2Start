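; A score pickup actor that bobs its sphere vertically and rewards the player on contact.
; A timeline started on BeginPlay drives the sphere's relative height.
; When BP_ThirdPersonCharacter overlaps the collision, it adds a random 11–19 (not the commented 5–10) to the Score on the level's BP_ProgPrac, found via GetActorOfClass.
; It then prints the new score and destroys itself.
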(event `self.ReceiveBeginPlay`
  (bind (_direction _keymovement) (`Timeline|KeyMovement`)
    (:`Update`
      (`SceneComponent.K2_SetRelativeLocation` (`self.Sphere`) (`KismetMathLibrary.MakeVector` 0.0 0.0 (+ (* _keymovement 100.0) 50.0)) false false))))

(event `self.Collision.OnComponentBeginOverlap`
  (params (OverlappedComponent :type "PrimitiveComponent Object Reference") (OtherActor :type "Actor Object Reference") (OtherComp :type "PrimitiveComponent Object Reference") (OtherBodyIndex :type Integer) (bFromSweep :type Boolean) (SweepResult :type "HitResult Structure (by ref)"))
  (cast `/Game/ThirdPerson/Blueprints/BP_ThirdPersonCharacter` OtherActor) ; Checks if the player ran into it
  (bind _returnvalue (`GameplayStatics.GetActorOfClass` "/Game/ProgPrac2/BP_ProgPrac.BP_ProgPrac_C")) ; find the bp_progprac that's in the level
  ;[1 1 1] Finding out what the score is and add between 5 and 10 and tells the player what their new score is
  (bind _output_get (set `/Game/ProgPrac2/BP_ProgPrac.Score` (+ (`/Game/ProgPrac2/BP_ProgPrac.Score` _returnvalue) (`KismetMathLibrary.RandomIntegerInRange` 11 19)) _returnvalue))
  (`KismetSystemLibrary.PrintString` (`KismetStringLibrary.Concat_StrStr` "Score: " (`KismetStringLibrary.Conv_IntToString` _output_get)))
  (`self.K2_DestroyActor`))

(fn `UserConstructionScript`)