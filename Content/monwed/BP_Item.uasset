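; BP_Item is an item actor with a physics Cube that can be picked up, dropped and used.
; Pickup disables the Cube's physics and collision, then snaps the actor to a named socket on the given parent actor.
; Drop only re-enables physics, without detaching or restoring collision.
; UsePrimary, noted as triggered by the character's left mouse button, is a print-only stub.
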(event `Pickup`
  (params (ParentActor :type "Actor Object Reference") (Mesh :type "SceneComponent Object Reference") (SocketName :type Name))
  (`PrimitiveComponent.SetSimulatePhysics` (`self.Cube`) false) ; Stop Simulating Physics
  (`PrimitiveComponent.SetCollisionEnabled` (`self.Cube`) "NoCollision")
  (`self.K2_AttachToActor` self ParentActor SocketName "SnapToTarget" "SnapToTarget" "KeepRelative" true))

(event `Drop`
  (`KismetSystemLibrary.PrintString` "Drop!")
  (`PrimitiveComponent.SetSimulatePhysics` (`self.Cube`) true) ; Start Simulating physics
)

(event `Use Primary`
  (`KismetSystemLibrary.PrintString` "UsePrimary"))

(fn `UserConstructionScript`)