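; BP_Enemy is a simple enemy Blueprint that announces itself on BeginPlay and loses health when its TakeDamage event fires.
; TakeDamage subtracts the damage and prints a red message that subtracts it again from the updated Health, so the shown value is lower than stored.
; It calls CheckIfAlive without using the result, then uses the pure Alivecheckpure to print a death message and destroy the actor once Health is not above zero.
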(event `self.ReceiveBeginPlay`
  (`KismetSystemLibrary.PrintString` "Hello, I have been programmed to destroy you."))

(event `TakeDamage`
  (params (by :type "Float (double-precision)" :default 0.2))
  (bind _returnvalue (- (`self.Health`) by))
  (set `self.Health` _returnvalue) ; make sure we lose that health
  (`KismetSystemLibrary.PrintString` (`KismetStringLibrary.Concat_StrStr` "Ouch! My Health is now " (`KismetStringLibrary.Conv_DoubleToString` _returnvalue)) true true (struct :`R` 0.900866 :`B` 0.105934 :`A` 1.0))
  (`self.CheckIfAlive` (`self.Health`))
  (if (not (`self.alivecheckpure` (`self.Health`)))
    (`KismetSystemLibrary.PrintString` "I am now dead")
    (`self.K2_DestroyActor`)))

(fn `alivecheckpure`
  (params (health :type "Float (double-precision)"))
  (returns (isAlive :type Boolean))
  (return (> health 0.0)))

(fn `CheckIfAlive`
  (params (Health :type "Float (double-precision)"))
  (returns (IsAlive :type Boolean))
  (return (> Health 0.0)))

(fn `UserConstructionScript`)